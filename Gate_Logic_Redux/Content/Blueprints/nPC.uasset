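; NPC actor that acts as a dialogue participant and starts a conversation when the player's Hero2p0 enters its box trigger.
; The overlap passes the hero's PlayerController and itself to the dialogue asset.
; Participant functions supply a name, icon and gender, while condition, value and event functions are stubs returning defaults.
; Ending overlap hides the hero's root component without propagating to children and clears InReach.
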(event `self.Box.OnComponentBeginOverlap`
  (params (OverlappedComponent :type "PrimitiveComponent Object Reference") (OtherActor :type "Actor Object Reference") (OtherComp :type "PrimitiveComponent Object Reference") (OtherBodyIndex :type Integer) (bFromSweep :type Boolean) (SweepResult :type "HitResult Structure (by ref)"))
  (bind _ashero_2p_0 (cast `/Game/Hero2p0` OtherActor))
  (bind _asplayer_controller (cast `PlayerController` (`Pawn.GetController` _ashero_2p_0)))
  (`DlgManager.StartDialogue2` (`self.dlgDialogue`) _asplayer_controller self))

(event `self.ReceiveActorEndOverlap`
  (params (OtherActor :type "Actor Object Reference"))
  (bind _ashero_2p_0 (cast `/Game/Hero2p0` OtherActor))
  (`SceneComponent.SetVisibility` (`Actor.RootComponent` _ashero_2p_0) false false)
  (set `self.inReach` false))

(fn `CheckCondition`
  (params (ConditionName :type "Name (by ref)"))
  (returns (ReturnValue :type Boolean))
  (return false))

(fn `GetBoolValue`
  (params (ValueName :type "Name (by ref)"))
  (returns (ReturnValue :type Boolean))
  (return false))

(fn `GetFloatValue`
  (params (ValueName :type "Name (by ref)"))
  (returns (ReturnValue :type "Float (double-precision)"))
  (return 0.0))

(fn `GetIntValue`
  (params (ValueName :type "Name (by ref)"))
  (returns (ReturnValue :type Integer))
  (return 0))

(fn `GetNameValue`
  (params (ValueName :type "Name (by ref)"))
  (returns (ReturnValue :type Name))
  (return "None"))

(fn `GetParticipantDisplayName`
  (params (ActiveSpeaker :type Name))
  (returns (ReturnValue :type Text))
  (return ""))

(fn `GetParticipantGender`
  (returns (ReturnValue :type "ETextGender Enum"))
  (return "Masculine"))

(fn `GetParticipantIcon`
  (params (ActiveSpeaker :type Name) (ActiveSpeakerState :type Name))
  (returns (ReturnValue :type "Texture2D Object Reference"))
  (return "/Game/Icons/740full-kevin-spacey.740full-kevin-spacey"))

(fn `GetParticipantName`
  (returns (ReturnValue :type Name))
  (return (`self.HisName`)))

(fn `ModifyBoolValue`
  (params (ValueName :type "Name (by ref)") (bNewValue :type Boolean))
  (returns (ReturnValue :type Boolean))
  (return false))

(fn `ModifyFloatValue`
  (params (ValueName :type "Name (by ref)") (bDelta :type Boolean) (Value :type "Float (double-precision)"))
  (returns (ReturnValue :type Boolean))
  (return false))

(fn `ModifyIntValue`
  (params (ValueName :type "Name (by ref)") (bDelta :type Boolean) (Value :type Integer))
  (returns (ReturnValue :type Boolean))
  (return false))

(fn `ModifyNameValue`
  (params (ValueName :type "Name (by ref)") (NameValue :type "Name (by ref)"))
  (returns (ReturnValue :type Boolean))
  (return false))

(fn `OnDialogueEvent`
  (params (EventName :type "Name (by ref)"))
  (returns (ReturnValue :type Boolean))
  (return false))

(fn `UserConstructionScript`)